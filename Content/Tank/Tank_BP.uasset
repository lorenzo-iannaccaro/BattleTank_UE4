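; Player-drivable tank pawn Blueprint that wires player input to movement, aiming, camera and firing components.
; On BeginPlay it hands turret, barrel and track components to TankAiming and TankMovement, then links itself to its health bar widget.
; Input drives tracks directly or through movement intents, rotates a gimbal and spring arm to aim the camera, toggles first- and third-person cameras, and fires via TankAiming.
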(event EventBeginPlay
  (Class|TankAimingComponent|InitialiseTurretandBarrel (Variables|Default|GetTankAiming) (Variables|Default|GetTankTurret) (Variables|Default|GetTankBarrel))
  (Class|TankMovementComponent|InitialiseTracks (Variables|Default|GetTankMovement1) (Variables|Default|GetTankTrackLeft) (Variables|Default|GetTankTrackRight))
  (CallFunction|InitializeHealthBarWidget))

(event Input|ActionEvents|InputActionFire
  (params (Key :type Key%20Structure :default "None"))
  ;[1 1 1] Fire input binding
  (:Pressed
    (Class|TankAimingComponent|Fire (Variables|Default|GetTankAiming))))

(event Input|ActionEvents|InputActionSwitchCamera
  (params (Key :type Key%20Structure :default "None"))
  ;[1 1 1] Switch camera input binding
  (:Pressed
    (Components|Activation|ToggleActive (Variables|Default|Get1st%20person%20camera))
    (Components|Activation|ToggleActive (Variables|Default|Get3rd%20person%20camera))))

(event Input|AxisEvents|InputAxisAimHorizontal
  (params (AxisValue :type Float%20%28single-precision%29))
  ;[1 1 1] Camera XY axis Input Binding
  (Transformation|AddLocalRotation (Variables|Default|GetHorizontalGimbal) (Math|Rotator|MakeRotator 0.0 0.0 (* AxisValue 1.0)) false false))

(event Input|AxisEvents|InputAxisAimVertical
  (params (AxisValue :type Float%20%28single-precision%29))
  ;[1 1 1] Camera XY axis Input Binding
  (Transformation|AddLocalRotation (Variables|Default|GetSpringArm) (Math|Rotator|MakeRotator 0.0 (* AxisValue 1.0) 0.0) false false))

(event Input|AxisEvents|InputAxisLeftTrackThrottle
  (params (AxisValue :type Float%20%28single-precision%29))
  ;[1 1 1] Tank movement input binding
  (Class|TankTrack|SetThrottle (Variables|Default|GetTankTrackLeft) AxisValue))

(event Input|AxisEvents|InputAxisRightTrackThrottle
  (params (AxisValue :type Float%20%28single-precision%29))
  ;[1 1 1] Tank movement input binding
  (Class|TankTrack|SetThrottle (Variables|Default|GetTankTrackRight) AxisValue))

(event Input|AxisEvents|InputAxisMoveForward
  (params (AxisValue :type Float%20%28single-precision%29))
  ;[1 1 1] Tank movement input binding
  (Class|TankMovementComponent|IntendMoveForward (Variables|Default|GetTankMovement1) AxisValue))

(event Input|AxisEvents|InputAxisTurnClockwise
  (params (AxisValue :type Float%20%28single-precision%29))
  ;[1 1 1] Tank movement input binding
  (Class|TankMovementComponent|IntendTurnClockwise (Variables|Default|GetTankMovement1) AxisValue))

(fn ConstructionScript)

(fn InitializeHealthBarWidget
  (bind _ashealth_bar_bp (Utilities|Casting|CastToHealthBar_BP (UserInterface|GetUserWidgetObject (Variables|Default|GetHealthWidget))))
  (Variables|/Game/UI/HealthBar_BP.HealthBar_BP_C|SetMyTank _ashealth_bar_bp self)
  (return))